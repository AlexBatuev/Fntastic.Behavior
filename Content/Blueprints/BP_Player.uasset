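; BP_Player is a player-controlled actor with movement, look controls and line-trace interaction.
; Movement axes drive input along the actor's forward and right vectors, while turn and look axes feed controller yaw and pitch.
; The Interaction action traces the Visibility channel a short distance forward from the camera and sends InteractionMessage to the hit actor.
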(event `InputAction|Interaction`
  (params (Key :type "Key Structure"))
  (bind _camera (`self.Camera`))
  (bind _returnvalue (`SceneComponent.K2_GetComponentLocation` _camera))
  ;[1 1 1] Interaction
  (:`Pressed`
    (bind (_outhit _returnvalue_2) (`KismetSystemLibrary.LineTraceSingle` _returnvalue (+ _returnvalue (* (`SceneComponent.GetForwardVector` _camera) 750.0)) "TraceTypeQuery1"))
    (if _returnvalue_2
      (message `/Game/Blueprints/BPI_Interaction.Interaction` (`.HitActor` (`GameplayStatics.BreakHitResult` _outhit))))))

(event `InputAxis|Turn` :overrideparent false
  (params (AxisValue :type "Float (single-precision)"))
  ;[1 1 1] LookAround
  (`self.AddControllerYawInput` AxisValue))

(event `InputAxis|MoveForward` :consume false :overrideparent false
  (params (AxisValue :type "Float (single-precision)"))
  ;[1 1 1] Movement
  (`self.AddMovementInput` (`self.GetActorForwardVector`) AxisValue))

(event `InputAxis|LookUp` :overrideparent false
  (params (AxisValue :type "Float (single-precision)"))
  ;[1 1 1] LookAround
  (`self.AddControllerPitchInput` AxisValue))

(event `InputAxis|MoveRight` :consume false :overrideparent false
  (params (AxisValue :type "Float (single-precision)"))
  ;[1 1 1] Movement
  (`self.AddMovementInput` (`self.GetActorRightVector`) AxisValue))

(fn `UserConstructionScript`)