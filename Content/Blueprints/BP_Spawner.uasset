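; BP_Spawner is a spawner actor that creates BP_Turtle actors at its own location.
; Its construction script applies the Color material to a cone and writes its Text value to a text render component.
; SpawnTurtle hands the spawner's Color, Collector and BehaviorTree to each new turtle, adjusting for collisions but always spawning.
; The event graph is empty, so spawning relies on an external call to SpawnTurtle.
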(fn `SpawnTurtle`
  (`|SpawnActorFromClass` "/Game/Blueprints/BP_Turtle.BP_Turtle_C" (`KismetMathLibrary.MakeTransform` (`self.K2_GetActorLocation`)) "AdjustIfPossibleButAlwaysSpawn" "OverrideRootScale" null (`self.Color`) (`self.Collector`) (`self.BehaviorTree`) null))

(fn `UserConstructionScript`
  (`PrimitiveComponent.SetMaterial` (`self.Cone`) 0 (`self.Color`))
  (`TextRenderComponent.K2_SetText` (`self.TextRender`) (`self.Text`)))