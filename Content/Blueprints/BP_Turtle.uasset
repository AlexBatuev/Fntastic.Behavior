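; BP_Turtle is an AI-driven turtle pawn that runs a behavior tree through its AIC_TurtleController.
; On BeginPlay it casts its controller to AIC_TurtleController and starts the turtle's own BehaviorTree variable on it.
; The construction script applies the Color material to its Cube component.
; A MoveBackward function adds movement input opposite the forward vector, with no caller in this Blueprint.
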(event `self.ReceiveBeginPlay`
  (bind _asaic_turtle_controller (cast `/Game/Blueprints/AIC_TurtleController` (`self.GetController`)))
  (`/Game/Blueprints/AIC_TurtleController.StartBehaviorTree` _asaic_turtle_controller (`self.BehaviorTree`)))

(fn `MoveBackward`
  (`self.AddMovementInput` (`self.GetActorForwardVector`) -1.0))

(fn `UserConstructionScript`
  (`PrimitiveComponent.SetMaterial` (`self.Cube`) 0 (`self.Color`)))