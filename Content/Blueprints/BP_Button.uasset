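; BP_Button is an interactable button that tells its linked Spawner to spawn a turtle.
; BeginPlay caches the start location and an offset target, and the construction script sets the label from the Text variable.
; On Interaction, a timeline moves the whole actor between the two locations using its Height track.
; An IsBusy flag blocks further presses until the animation finishes.
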(event `self.ReceiveBeginPlay`
  ;[1 1 1] Init
  (set `self.InintialLocation` (`self.K2_GetActorLocation`))
  (set `self.AnimLocation` (+ (`self.InintialLocation`) (`self.AnimOffset`))))

(event `/Game/Blueprints/BPI_Interaction.Interaction`
  ;[1 1 1] Interaction
  (if (not (`self.IsBusy`))
    (`/Game/Blueprints/BP_Spawner.SpawnTurtle` (`self.Spawner`))
    (set `self.IsBusy` true)
    (bind (_direction _height) (`Timeline|AnimTimeline` :!via `PlayFromStart`)
      (:`Update`
        (`self.K2_SetActorLocation` (`KismetMathLibrary.VLerp` (`self.InintialLocation`) (`self.AnimLocation`) _height)))
      (:`Finished`
        (set `self.IsBusy` false)))))

(fn `UserConstructionScript`
  (`TextRenderComponent.K2_SetText` (`self.TextRender`) (`self.Text`)))